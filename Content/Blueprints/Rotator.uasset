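; Rotator is an actor that starts orbiting the player character once any actor overlaps it, and never stops.
; Each Tick flattens its offset from the player onto the horizontal plane, fixes it to a set radius and yaws it by a DeltaSeconds-scaled step.
; It moves to that offset at the player's height without sweeping, then builds its rotation from axes to face outward, away from the player.
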(event `self.ReceiveActorBeginOverlap`
  (params (OtherActor :type "Actor Object Reference"))
  (set `self.NewVar` true))

(event `self.ReceiveTick`
  (params (DeltaSeconds :type "Float (single-precision)"))
  (bind _returnvalue (`self.K2_GetActorLocation` (`GameplayStatics.GetPlayerCharacter` 0)))
  (bind _returnvalue_2 (`KismetMathLibrary.GreaterGreater_VectorRotator` (* (`KismetMathLibrary.Normal` (`KismetMathLibrary.ProjectPointOnToPlane` (- (`self.K2_GetActorLocation`) _returnvalue) (0.0 0.0 0.0) (0.0 0.0 1.0))) 300.0) (`KismetMathLibrary.MakeRot` 0.0 (* DeltaSeconds 90.0))))
  ;[1 1 1] Orbital
  (if (`self.NewVar`)
    (`self.K2_SetActorLocation` (+ _returnvalue_2 _returnvalue))
    (`self.SetActorRotation` (`KismetMathLibrary.MakeRotationFromAxes` _returnvalue_2 (`KismetMathLibrary.GreaterGreater_VectorRotator` _returnvalue_2 (`KismetMathLibrary.MakeRot` 0.0 90.0)) (0.0 0.0 1.0)))))

(fn `UserConstructionScript`)