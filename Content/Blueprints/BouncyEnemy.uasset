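; BouncyEnemy is an enemy actor that hops toward the player using physics and damages them on contact.
; Each mesh hit, except against another BouncyEnemy, turns it to face player 0 and overwrites its linear velocity with a push toward them plus an upward kick.
; Actor hits tagged Projectile reduce Health, ending in an explosion and destruction, while hits tagged Player apply damage to the player character.
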(event `self.StaticMesh2.OnComponentHit`
  (params (OtherActor :type "Actor Object Reference") (OtherComp :type "PrimitiveComponent Object Reference") (NormalImpulse :type "Object.Vector Structure") (Hit :type "EngineTypes.HitResult Structure (by ref)"))
  (bind _returnvalue (`KismetMathLibrary.FindLookAtRotation` (`self.K2_GetActorLocation`) (`self.K2_GetActorLocation` (`GameplayStatics.GetPlayerCharacter` 0))))
  (cast `/Game/Blueprints/BouncyEnemy` OtherActor
    (:`CastFailed`
      (`self.SetActorRotation` _returnvalue)
      (`PrimitiveComponent.SetPhysicsLinearVelocity` (+ (* (`KismetMathLibrary.Normal` (`KismetMathLibrary.GetForwardVector` _returnvalue)) 300.0) (0.0 0.0 600.0))))))

(event `self.ReceiveHit`
  (params (MyComp :type "PrimitiveComponent Object Reference") (Other :type "Actor Object Reference") (OtherComp :type "PrimitiveComponent Object Reference") (bSelfMoved :type Boolean) (HitLocation :type "Object.Vector Structure") (HitNormal :type "Object.Vector Structure") (NormalImpulse :type "Object.Vector Structure") (Hit :type "EngineTypes.HitResult Structure (by ref)"))
  (bind _health (`self.Health`))
  ;[1 1 1] Take Damage on Hit
  (if (`self.ActorHasTag` Other "Projectile")
    (set `self.Health` (- _health 1.0))
    (if (<= _health 0.0)
      (`GameplayStatics.SpawnEmitterAtLocation` "/Game/StarterContent/Particles/P_Explosion.P_Explosion" (`SceneComponent.K2_GetComponentLocation`))
      (`self.K2_DestroyActor`))
    (elif (`self.ActorHasTag` Other "Player")
      (`GameplayStatics.ApplyDamage` (`GameplayStatics.GetPlayerCharacter` 0) 1.1))))

(fn `UserConstructionScript`)